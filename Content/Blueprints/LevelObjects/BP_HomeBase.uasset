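; BP_HomeBase is the home base actor whose health decides game over.
; Damage lowers health, updates the commander's widget and plays a rate-limited alarm sound, or calls GameOver on GM_MissionControl when health runs out.
; Functions activate child-actor electric walls or turrets selected by a direction index.
; GetRandomAttackPoint returns only a zero vector, and the older HUD and random wall-activation loop are disconnected.
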(event `self.ReceiveBeginPlay`
  (set `self.Health` (`self.StartingHealth`))
  (`KismetSystemLibrary.Delay` 0.2)
  (bind _returnvalue (`GameplayStatics.GetActorOfClass` "/Game/Blueprints/Players/BP_Commander.BP_Commander_C"))
  (bind _output_get (set `self.Commander Widget` (`/Game/Blueprints/Players/BP_Commander.Commander Widget` _returnvalue)))
  (`/Game/UI/WBP_CommanderTest.SetBaseHealth` _output_get (`self.Health`) (`self.StartingHealth`)))

(event `self.ReceiveAnyDamage`
  (params (Damage :type "Float (single-precision)") (DamageType :type "DamageType Object Reference") (InstigatedBy :type "Controller Object Reference") (DamageCauser :type "Actor Object Reference"))
  (bind _output_get (set `self.Health` (- (`self.Health`) Damage)))
  (if (<= _output_get 0.0)
    (bind _asgm_mission_control (cast `/Game/Blueprints/GameModes/GM_MissionControl` (`GameplayStatics.GetGameMode`)))
    (`/Game/Blueprints/GameModes/GM_MissionControl.GameOver` _asgm_mission_control)
    (else
      (`/Game/UI/WBP_CommanderTest.SetBaseHealth` (`self.Commander Widget`) (`self.Health`) (`self.StartingHealth`))
      (if (`self.PlayAlarm`)
        (`GameplayStatics.PlaySoundAtLocation` "/Game/SFX/alarm_Cue.alarm_Cue" (`SceneComponent.K2_GetComponentLocation` (`self.AlarmLocation`)) (struct) 1.0 1.0 0.0 null null null null)
        (set `self.PlayAlarm` false)
        (`KismetSystemLibrary.Delay` 5.0)
        (set `self.PlayAlarm` true)))))

(fn `ActivateElectricWall`
  (params (NESW :type Integer))
  (locals (WallToUse :type "ChildActorComponent Object Reference"))
  (switch `int` NESW
    (:`Default`
      (set `local.WallToUse` (`self.BP_ElectricWall4`) :!label _label))
    (:`0`
      (set `local.WallToUse` (`self.BP_ElectricWall2`)))
    (:`1`
      (set `local.WallToUse` (`self.BP_ElectricWall3`)))
    (:`2`
      (goto _label))
    (:`3`
      (set `local.WallToUse` (`self.BP_ElectricWall1`))))
  (bind _asbp_electric_wall (cast `/Game/Blueprints/Defenses/BP_ElectricWall` (`ChildActorComponent.ChildActor` (`local.WallToUse`))))
  (`/Game/Blueprints/Defenses/BP_ElectricWall.ActivateWall` _asbp_electric_wall))

(fn `ActivateTurret`
  (params (NESW :type Integer))
  (locals (TurretToUse :type "ChildActorComponent Object Reference"))
  (switch `int` NESW
    (:`Default`
      (set `local.TurretToUse` (`self.BP_Turret3`) :!label _label))
    (:`0`
      (set `local.TurretToUse` (`self.BP_Turret`)))
    (:`1`
      (set `local.TurretToUse` (`self.BP_Turret1`)))
    (:`2`
      (set `local.TurretToUse` (`self.BP_Turret2`)))
    (:`3`
      (goto _label)))
  (bind _asbp_turret (cast `/Game/grant/BP_Turret` (`ChildActorComponent.ChildActor` (`local.TurretToUse`))))
  (`/Game/grant/BP_Turret.ActivateTurret` _asbp_turret))

(fn `Get Random Attack Point`
  (returns (Location :type "Vector Structure"))
  (return (0.0 0.0 0.0)))

(fn `UserConstructionScript`)