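; Level actor that flies an airplane over the map to deliver airdrops to a lettered and numbered grid cell.
; Airdrop starts the plane at a random horizontal offset from the center, aimed at the cell; only Supply is handled, and BeginPlay triggers one.
; Tick moves the plane, hides it when far from center and not dropping, and spawns a BP_PickupAirdrop with the chosen supply upon nearing the target.
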(event `self.ReceiveBeginPlay`
  (bind (_returnvalue_x _returnvalue_y _returnvalue_z) (`KismetMathLibrary.BreakVector` (`self.K2_GetActorLocation`)))
  (bind (_a0_x _a0_y) (`KismetMathLibrary.BreakVector` (`self.A0`)))
  (bind (_centerpoint_x _centerpoint_y) (`KismetMathLibrary.BreakVector` (`self.Centerpoint`)))
  (bind _output_get (set `self.ZCoord` _returnvalue_z))
  (set `self.A0` (`KismetMathLibrary.MakeVector` _a0_x _a0_y _output_get))
  (set `self.Centerpoint` (`KismetMathLibrary.MakeVector` _centerpoint_x _centerpoint_y _output_get))
  (`self.Airdrop` "NewEnumerator1" "NewEnumerator1" 7))

(event `self.ReceiveTick`
  (params (DeltaSeconds :type "Float (single-precision)"))
  (bind _airplane (`self.Airplane`))
  (bind _returnvalue (`SceneComponent.K2_GetComponentLocation` _airplane))
  (if (or (`self.Dropping`) (< (`KismetMathLibrary.Vector_Distance` _returnvalue (`self.Centerpoint`)) 20000.0))
    (`SceneComponent.SetVisibility` _airplane true true)
    (else
      (`SceneComponent.SetVisibility` _airplane false true)))
  (`SceneComponent.K2_SetWorldLocation` _airplane (+ _returnvalue (* (`self.AirplaneDirection`) (* DeltaSeconds 2500.0))) false false)
  (if (`self.Dropping`)
    (if (< (`KismetMathLibrary.Vector_Distance` (`SceneComponent.K2_GetComponentLocation` (`self.AirplaneModel`)) (`self.DropLocation`)) 50.0)
      (bind _returnvalue_2 (`|SpawnActorFromClass` (`self.ThingToDrop`) (`KismetMathLibrary.MakeTransform` (`self.DropLocation`)) "Undefined" "MultiplyWithRoot" null null))
      (bind _asbp_pickup_airdrop (cast `/Game/Blueprints/Airdrops/BP_PickupAirdrop` _returnvalue_2)
        (:`then`
          (set `/Game/Blueprints/Airdrops/BP_PickupAirdrop.ItemToDrop` (`self.Supplytype`) _asbp_pickup_airdrop))
        (:`CastFailed`
          _))
      (set `self.Dropping` false))))

(fn `Airdrop`
  (params (`Airdrop Type` :type "/Game/Data/AirdropType Enum" :default "NewEnumerator0") (`Location Letter` :type "/Game/Data/LocationLetters Enum" :default "NewEnumerator0") (`Location Number` :type Integer) (`Artillery Type` :type "/Game/Data/ArtilleryType Enum" :default "NewEnumerator0") (SupplyDropType :type "/Game/Data/SupplyDropType Enum" :default "NewEnumerator0"))
  (bind (_returnvalue_x _returnvalue_y) (`KismetMathLibrary.BreakVector` (`KismetMathLibrary.RandomUnitVector`)))
  ;[1 1 1] Select actor to drop
  (switch `/Game/Data/AirdropType` `Airdrop Type`
    (:`NewEnumerator1`
      (set `self.Supplytype` (`BlueprintMapLibrary.Map_Find` (`self.SuppliesMap`) SupplyDropType))
      (set `self.ThingToDrop` "/Game/Blueprints/Airdrops/BP_PickupAirdrop.BP_PickupAirdrop_C")
      (`SceneComponent.K2_SetWorldLocation` (`self.Airplane`) (+ (`self.Centerpoint`) (* (`KismetMathLibrary.Normal` (`KismetMathLibrary.MakeVector` _returnvalue_x _returnvalue_y)) 10000.0)) false false)
      (set `self.Dropping` true)
      (bind _output_get (set `self.DropLocation` (+ (`self.A0`) (`KismetMathLibrary.MakeVector` (* (`local.Location Number`) 100.0) (* (`KismetMathLibrary.Conv_ByteToInt` (`local.Location Letter`)) 100.0)))))
      (bind _output_get_2 (set `self.AirplaneDirection` (`KismetMathLibrary.Normal` (- _output_get (`SceneComponent.K2_GetComponentLocation` (`self.AirplaneModel`))))))
      (`SceneComponent.K2_SetWorldRotation` (`self.Airplane`) (`KismetMathLibrary.Conv_VectorToRotator` _output_get_2) false false))))

(fn `UserConstructionScript`)