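; GM_MissionControl is a game mode for a two-player local game pairing a first-person character with a commander.
; On BeginPlay it creates a second local player, spawns BP_FPSCharacter and BP_Commander at PlayerStart transforms and possesses them with controllers 0 and 1.
; It also prints all connected input devices.
; FPSPlayerDied triggers a five-second delayed respawn and repossession of the FPS character.
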(event `self.ReceiveBeginPlay`
  (`GameplayStatics.CreatePlayer` 1)
  (bind _returnvalue (`GameplayStatics.GetActorOfClass` "/Script/Engine.PlayerStart"))
  (bind _returnvalue_2 (`|SpawnActorFromClass` "/Game/Blueprints/Players/BP_FPSCharacter.BP_FPSCharacter_C" (`self.GetTransform` _returnvalue) "Undefined" "MultiplyWithRoot" null null))
  (`Controller.Possess` (`GameplayStatics.GetPlayerController` 0) _returnvalue_2)
  (bind _outactors (`GameplayStatics.GetAllActorsOfClass` "/Script/Engine.PlayerStart"))
  (bind _returnvalue_3 (`|SpawnActorFromClass` "/Game/Blueprints/Players/BP_Commander.BP_Commander_C" (`self.GetTransform` (`|GetArrayItem` _outactors 1)) "Undefined" "MultiplyWithRoot" null null))
  (`Controller.Possess` (`GameplayStatics.GetPlayerController` 1) _returnvalue_3)
  (bind _outinputdevices (`InputDeviceLibrary.GetAllConnectedInputDevices`))
  (for _array_element _outinputdevices
    (`KismetSystemLibrary.PrintString` (`KismetStringLibrary.Conv_InputDeviceIdToString` _array_element) true true (struct :`R` 1.0 :`B` 0.640301 :`A` 1.0))))

(event `RespawnPlayerDelay`
  (`KismetSystemLibrary.Delay` 5.0)
  (bind _returnvalue (`GameplayStatics.GetActorOfClass` "/Script/Engine.PlayerStart"))
  (bind _returnvalue_2 (`|SpawnActorFromClass` "/Game/Blueprints/Players/BP_FPSCharacter.BP_FPSCharacter_C" (`self.GetTransform` _returnvalue) "Undefined" "MultiplyWithRoot" null null))
  (`Controller.Possess` (`GameplayStatics.GetPlayerController` 0) _returnvalue_2))

(fn `FPSPlayerDied`
  (`self.RespawnPlayerDelay`))

(fn `UserConstructionScript`)