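; Airdrop fire missile actor that explodes on impact and leaves a temporary zone that sets enemies on fire.
; When the static mesh hits, it stops simulating, hides, spawns an explosion, silences its audio and turns on the box's visibility and overlap events.
; BP_Enemy actors that begin overlapping the box get SetOnFire until the actor destroys itself after a delay.
; An unconnected leftover area-damage loop never runs.
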(event `self.StaticMesh.OnComponentHit`
  (params (HitComponent :type "PrimitiveComponent Object Reference") (OtherActor :type "Actor Object Reference") (OtherComp :type "PrimitiveComponent Object Reference") (NormalImpulse :type "Vector Structure") (Hit :type "HitResult Structure (by ref)"))
  (bind _staticmesh (`self.StaticMesh`))
  (bind _box (`self.Box`))
  (`PrimitiveComponent.SetSimulatePhysics` _staticmesh false)
  (`PrimitiveComponent.SetCollisionEnabled` (`self.StaticMesh`) "NoCollision")
  (`SceneComponent.SetVisibility` _staticmesh false true)
  (`SceneComponent.SetVisibility` _box true true)
  (set `PrimitiveComponent.bGenerateOverlapEvents` true _box)
  (`NiagaraFunctionLibrary.SpawnSystemAtLocation` "/Niagara/DefaultAssets/Templates/Systems/SimpleExplosion.SimpleExplosion" (`SceneComponent.K2_GetComponentLocation` (`self.explosionPoint`)) (struct) (5.0 5.0 5.0))
  (`AudioComponent.Stop` (`self.Audio`))
  (`KismetSystemLibrary.Delay` 22.0)
  (`self.K2_DestroyActor`))

(event `self.Box.OnComponentBeginOverlap`
  (params (OverlappedComponent :type "PrimitiveComponent Object Reference") (OtherActor :type "Actor Object Reference") (OtherComp :type "PrimitiveComponent Object Reference") (OtherBodyIndex :type Integer) (bFromSweep :type Boolean) (SweepResult :type "HitResult Structure (by ref)"))
  (bind _asbp_enemy (cast `/Game/Blueprints/Enemies/BP_Enemy` OtherActor))
  (`/Game/Blueprints/Enemies/BP_Enemy.SetOnFire` _asbp_enemy))

(fn `UserConstructionScript`)