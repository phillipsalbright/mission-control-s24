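; Player pawn for the commander role, who looks around within clamped angles, clicks world widgets and manages a money balance.
; Enhanced Input pans and zooms an orthographic scene capture view and simulates mouse clicks through a WidgetInteraction component.
; Purchase and income functions update the balance and push it to two widget-component displays.
; Possession adds a crosshair for player index 1, and in single-player a swap input possesses the FPS character.
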(event `self.ReceiveBeginPlay`
  (bind _moneycount (`self.moneyCount`))
  (bind _aswbp_commander_test (cast `/Game/UI/WBP_CommanderTest` (`WidgetComponent.GetWidget` (`self.Widget`))))
  (bind _output_get (set `self.Commander Widget` _aswbp_commander_test))
  (`/Game/UI/WBP_CommanderTest.MoneyChanged` _output_get _moneycount)
  (bind _aswbp_money_display (cast `/Game/UI/WBP_MoneyDisplay` (`WidgetComponent.GetWidget` (`self.Widget2`))))
  (set `self.As WBP Money Display` _aswbp_money_display)
  (`/Game/UI/WBP_MoneyDisplay.MoneyChanged` _aswbp_money_display _moneycount))

(event `self.ReceivePossessed`
  (params (NewController :type "Controller Object Reference"))
  (bind _asplayer_controller (cast `PlayerController` NewController))
  (bind _returnvalue (pcsubsystem `EnhancedInputLocalPlayerSubsystem` _asplayer_controller))
  (`/Engine/EditorBlueprintResources/StandardMacros.IsValid` _returnvalue
    (:`Is Valid`
      (`EnhancedInputSubsystemInterface.AddMappingContext` _returnvalue "/Game/FirstPerson/Input/IMC_Commander.IMC_Commander" 0 (struct))
      (bind _returnvalue_2 (`|CreateWidget` "/Game/UI/WBP_CommanderCrosshair.WBP_CommanderCrosshair_C" (`GameplayStatics.GetPlayerController` 1)))
      (`UserWidget.AddToPlayerScreen` _returnvalue_2 0))))

(event `EnhancedInput|/Game/FirstPerson/Input/Actions/IA_Look`
  (params (ActionValue :type "Vector2D Structure") (ElapsedSeconds :type "Float (double-precision)") (TriggeredSeconds :type "Float (double-precision)") (InputAction :type "InputAction Object Reference" :default "/Game/FirstPerson/Input/Actions/IA_Look.IA_Look"))
  (bind _returnvalue (`GameplayStatics.GetWorldDeltaSeconds`))
  (bind _camera (`self.Camera`))
  (bind (_relativerotation_roll _relativerotation_pitch _relativerotation_yaw) (`KismetMathLibrary.BreakRotator` (`SceneComponent.RelativeRotation` _camera)))
  (:`Triggered`
    (`SceneComponent.K2_SetRelativeRotation` _camera (`KismetMathLibrary.MakeRotator` 0.0 (`KismetMathLibrary.FClamp` (+ _relativerotation_pitch (* _returnvalue ActionValue_Y -35.0)) -30.0 30.0) (`KismetMathLibrary.FClamp` (+ _relativerotation_yaw (* _returnvalue ActionValue_X 40.0)) -35.0 50.0)) false false)))

(event `EnhancedInput|/Game/FirstPerson/Input/Actions/IA_Shoot`
  (params (ActionValue :type Boolean) (ElapsedSeconds :type "Float (double-precision)") (TriggeredSeconds :type "Float (double-precision)") (InputAction :type "InputAction Object Reference" :default "/Game/FirstPerson/Input/Actions/IA_Shoot.IA_Shoot")))

(event `EnhancedInput|/Game/FirstPerson/Input/Actions/IA_Select`
  (params (ActionValue :type Boolean) (ElapsedSeconds :type "Float (double-precision)") (TriggeredSeconds :type "Float (double-precision)") (InputAction :type "InputAction Object Reference" :default "/Game/FirstPerson/Input/Actions/IA_Select.IA_Select"))
  (bind _widgetinteraction (`self.WidgetInteraction`))
  (:`Started`
    (`WidgetInteractionComponent.PressPointerKey` _widgetinteraction "LeftMouseButton")
    (`KismetSystemLibrary.DelayUntilNextTick`)
    (`WidgetInteractionComponent.ReleasePointerKey` _widgetinteraction "LeftMouseButton")))

(event `EnhancedInput|/Game/FirstPerson/Input/Actions/IA_SwapPlayer`
  (params (ActionValue :type Boolean) (ElapsedSeconds :type "Float (double-precision)") (TriggeredSeconds :type "Float (double-precision)") (InputAction :type "InputAction Object Reference" :default "/Game/FirstPerson/Input/Actions/IA_SwapPlayer.IA_SwapPlayer"))
  (bind _returnvalue (`self.GetController`))
  (:`Started`
    (bind _returnvalue_2 (`GameplayStatics.LoadGameFromSlot` "PlayerSetting"))
    (bind _asbp_player_setting (cast `/Game/Data/BP_PlayerSetting` _returnvalue_2))
    (if (`/Game/Data/BP_PlayerSetting.SinglePlayer` _asbp_player_setting)
      (bind _returnvalue_3 (`GameplayStatics.GetActorOfClass` "/Game/Blueprints/Players/BP_FPSCharacter.BP_FPSCharacter_C"))
      (bind _asplayer_controller (cast `PlayerController` _returnvalue))
      (bind _returnvalue_4 (pcsubsystem `EnhancedInputLocalPlayerSubsystem` _asplayer_controller))
      (`/Engine/EditorBlueprintResources/StandardMacros.IsValid` _returnvalue_4
        (:`Is Valid`
          (message `EnhancedInputSubsystemInterface.RemoveMappingContext` _returnvalue_4 "/Game/FirstPerson/Input/IMC_Commander.IMC_Commander" (make `ModifyContextOptions` true))
          (`Controller.Possess` _returnvalue _returnvalue_3))))))

(event `EnhancedInput|/Game/FirstPerson/Input/Actions/IA_Exit`
  (params (ActionValue :type Boolean) (ElapsedSeconds :type "Float (double-precision)") (TriggeredSeconds :type "Float (double-precision)") (InputAction :type "InputAction Object Reference" :default "/Game/FirstPerson/Input/Actions/IA_Exit.IA_Exit"))
  (:`Started`
    (`GameplayStatics.OpenLevelBySoftObjectPtr` "/Game/Maps/MainMenu.MainMenu")))

(event `EnhancedInput|/Game/FirstPerson/Input/Actions/IA_Move`
  (params (ActionValue :type "Vector2D Structure") (ElapsedSeconds :type "Float (double-precision)") (TriggeredSeconds :type "Float (double-precision)") (InputAction :type "InputAction Object Reference" :default "/Game/FirstPerson/Input/Actions/IA_Move.IA_Move"))
  (bind _scene (`self.Scene`))
  (bind (_returnvalue_x _returnvalue_y _returnvalue_z) (`KismetMathLibrary.BreakVector` (+ (`SceneComponent.K2_GetComponentLocation` _scene) (`KismetMathLibrary.MakeVector` (* ActionValue_X (`GameplayStatics.GetWorldDeltaSeconds`) -1500.0) (* ActionValue_Y (`GameplayStatics.GetWorldDeltaSeconds`) 1500.0)))))
  (:`Triggered`
    (`SceneComponent.K2_SetWorldLocation` _scene (`KismetMathLibrary.MakeVector` (`KismetMathLibrary.FClamp` _returnvalue_x -10000.0 10000.0) (`KismetMathLibrary.FClamp` _returnvalue_y -10000.0 10000.0) _returnvalue_z) false false)))

(event `EnhancedInput|/Game/FirstPerson/Input/Actions/IA_Zoom`
  (params (ActionValue :type "Float (double-precision)") (ElapsedSeconds :type "Float (double-precision)") (TriggeredSeconds :type "Float (double-precision)") (InputAction :type "InputAction Object Reference" :default "/Game/FirstPerson/Input/Actions/IA_Zoom.IA_Zoom"))
  (bind _scenecapturecomponent2d (`self.SceneCaptureComponent2D`))
  (:`Triggered`
    (set `SceneCaptureComponent2D.OrthoWidth` (`KismetMathLibrary.FClamp` (+ (`SceneCaptureComponent2D.OrthoWidth` _scenecapturecomponent2d) (* ActionValue (`GameplayStatics.GetWorldDeltaSeconds`) 420.0)) 350.0 4500.0) _scenecapturecomponent2d)))

(fn `AddCurrency`
  (params (Money :type Integer))
  (bind _output_get (set `self.moneyCount` (+ (`self.moneyCount`) Money)))
  (`/Game/UI/WBP_CommanderTest.MoneyChanged` (`self.Commander Widget`) _output_get)
  (`/Game/UI/WBP_MoneyDisplay.MoneyChanged` (`self.As WBP Money Display`) _output_get))

(fn `Buy Attempt`
  (params (Balance :type Integer) (Cost :type Integer))
  (returns (didBuy :type Boolean))
  (set `self.bought` false)
  (`/Engine/EditorBlueprintResources/StandardMacros.CompareInt` Balance Cost
    (:`>`
      (`KismetSystemLibrary.PrintString` "commander buy request success" :!label _label)
      (bind _output_get (set `self.moneyCount` (- Balance Cost)))
      (`/Game/UI/WBP_CommanderTest.MoneyChanged` (`self.Commander Widget`) _output_get)
      (`/Game/UI/WBP_MoneyDisplay.MoneyChanged` (`self.As WBP Money Display`) _output_get)
      (bind _output_get_2 (set `self.bought` true)))
    (:`==`
      (goto _label))
    (:`<`
      (`KismetSystemLibrary.PrintString` "commander is too broke to buy")))
  (return _output_get_2))

(fn `Can Buy Check`
  (params (balance :type Integer) (cost :type Integer))
  (returns (canbuy :type Boolean))
  (`/Engine/EditorBlueprintResources/StandardMacros.CompareInt` balance cost
    (:`>`
      _)
    (:`==`
      _)
    (:`<`
      (return false)))
  (return true))

(fn `UserConstructionScript`)