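; BP_InventoryComponent is a player component that holds a list of weapons and tracks which one is equipped.
; It adds weapons to the list, equips the first, and forwards shooting to the equipped weapon with debug prints.
; Switching unequips the current weapon and equips the next with wrap-around indexing.
; It falls back to the first weapon when the equipped one is invalid or missing from the list.
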(fn `AddWeapon`
  (params (NewWeapon :type "/Game/Blueprints/Weapons/BP_Weapon Object Reference"))
  (`KismetArrayLibrary.Array_Add` (`self.Weapons`) NewWeapon))

(fn `EquipFirstWeapon`
  (bind _output (`|GetArrayItem` (`self.Weapons`)))
  (if (`KismetSystemLibrary.IsValid` _output)
    (`/Game/Blueprints/Weapons/BP_Weapon.Equip` _output)
    (set `self.EquippedWeapon` _output)))

(fn `EquipNextWeapon`
  (bind _equippedweapon (`self.EquippedWeapon`))
  (bind _weapons (`self.Weapons`))
  (bind _returnvalue (`KismetArrayLibrary.Array_Find` _weapons _equippedweapon))
  (if (`KismetSystemLibrary.IsValid` _equippedweapon)
    (if (< _returnvalue 0)
      (`self.EquipFirstWeapon` :!label _label)
      (else
        (`/Game/Blueprints/Weapons/BP_Weapon.Unequip` (`self.EquippedWeapon`))
        (bind _output_get (set `self.EquippedWeapon` (`|GetArrayItem` _weapons (mod (+ _returnvalue 1) (`KismetArrayLibrary.Array_Length` _weapons)))))
        (`/Game/Blueprints/Weapons/BP_Weapon.Equip` _output_get)))
    (else
      (goto _label))))

(fn `ShootEquippedWeapon`
  (bind _equippedweapon (`self.EquippedWeapon`))
  (if (`KismetSystemLibrary.IsValid` _equippedweapon)
    (`/Game/Blueprints/Weapons/BP_Weapon.Shoot` _equippedweapon)
    (`KismetSystemLibrary.PrintString` "shooted")
    (else
      (`KismetSystemLibrary.PrintString` "pooted"))))