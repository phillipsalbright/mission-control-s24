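; AI controller for the spider enemy, which assaults attack points by the home base and hunts the player on sight.
; On possess it heads for a random BP_AttackPoint and caches BP_HomeBase, or, lacking points, moves toward the player after a delay.
; Perception sets or clears the player as Target.
; Tick drives behavior without a behavior tree: chase and attack Target, otherwise reach the attack point, face the base and attack.
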(event `self.ReceivePossess`
  (params (PossessedPawn :type "Pawn Object Reference"))
  (bind _asbp_enemy (cast `/Game/Blueprints/Enemies/BP_Enemy` PossessedPawn))
  (set `self.As BP Enemy` _asbp_enemy)
  (bind _outactors (`GameplayStatics.GetAllActorsOfClass` "/Game/Blueprints/BP_AttackPoint.BP_AttackPoint_C"))
  (if (> (`KismetArrayLibrary.Array_Length` _outactors) 0)
    (bind _output_get (set `self.AttackPoint` (`KismetArrayLibrary.Array_Random` _outactors)))
    (`|AIMoveTo` PossessedPawn (0.0 0.0 0.0) _output_get
      (:`then`
        (set `self.Target` null)
        (bind _returnvalue (`GameplayStatics.GetActorOfClass` "/Game/Blueprints/BP_HomeBase.BP_HomeBase_C"))
        (set `self.HomeBase` _returnvalue)))
    (else
      (`KismetSystemLibrary.Delay` 12.0)
      (bind _returnvalue_2 (`GameplayStatics.GetActorOfClass` "/Game/Blueprints/Players/BP_FPSCharacter.BP_FPSCharacter_C"))
      (`|AIMoveTo` PossessedPawn (0.0 0.0 0.0) _returnvalue_2))))

(event `self.AIPerception.OnPerceptionUpdated`
  (params (UpdatedActors :type "Array of Actor Object Reference (by ref)")))

(event `self.AIPerception.OnTargetPerceptionInfoUpdated`
  (params (UpdateInfo :type "ActorPerceptionUpdateInfo Structure (by ref)"))
  (bind _asbp_fpscharacter (cast `/Game/Blueprints/Players/BP_FPSCharacter` UpdateInfo_Target))
  (if (`.bSuccessfullySensed` (break `AIStimulus` (`.Stimulus` (break `ActorPerceptionUpdateInfo` UpdateInfo))))
    (set `self.Target` _asbp_fpscharacter)
    (else
      (set `self.Target` null))))

(event `self.ReceiveTick`
  (params (DeltaSeconds :type "Float (single-precision)"))
  (bind _returnvalue (`self.K2_GetPawn`))
  (bind _target (`self.Target`))
  (bind _homebase (`self.HomeBase`))
  (bind _returnvalue_2 (`self.K2_GetActorLocation` _returnvalue))
  (bind _returnvalue_3 (`KismetMathLibrary.FindLookAtRotation` (`self.K2_GetActorLocation` _returnvalue) (`self.K2_GetActorLocation` _homebase)))
  (if (`KismetSystemLibrary.IsValid` _returnvalue)
    (if (`KismetSystemLibrary.IsValid` _target)
      (if (< (`KismetMathLibrary.VSize` (- _returnvalue_2 (`self.K2_GetActorLocation` _target))) 200.0)
        (`/Game/Blueprints/Enemies/BP_Enemy.Attack` (`self.As BP Enemy`) :!label _label)
        (else
          (`|AIMoveTo` _returnvalue (0.0 0.0 0.0) _target 120.0)))
      (elif (< (`KismetMathLibrary.Vector_Distance` _returnvalue_2 (`self.K2_GetActorLocation` (`self.AttackPoint`))) 100.0)
        (if (`KismetSystemLibrary.IsValid` _homebase)
          (`self.SetControlRotation` _returnvalue_3)
          (`self.K2_SetActorRotation` _returnvalue _returnvalue_3 false)
          (goto _label)
          (else
            (goto _label)))
        (else
          (`|AIMoveTo` _returnvalue (0.0 0.0 0.0) (`self.AttackPoint`) 10.0
            (:`then`
              (set `self.Target` null))))))))

(event `self.ReceiveUnPossess`
  (params (UnpossessedPawn :type "Pawn Object Reference"))
  (set `self.bAutoDestroyWhenFinished` true))

(fn `UserConstructionScript`)