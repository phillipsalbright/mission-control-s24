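; BP_ExplodingSpider is a suicide-bomber spider enemy that plays montages when it spawns and when it takes damage.
; Its Attack override fires once, guarded by an Exploded flag, halting movement and starting the explosion event.
; After a short delay, the explosion damages every non-BP_Enemy actor overlapping its capsule.
; Death is called inside that damage loop, so it runs per victim and not at all without one.
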(event `self.ReceiveBeginPlay`
  (`parent.ReceiveBeginPlay`)
  (`|PlayMontage` (`self.Mesh`) "/Game/SpiderMinion/Animations/Anim_Enter_Montage.Anim_Enter_Montage"))

(event `self.ReceiveTick`
  (params (DeltaSeconds :type "Float (single-precision)"))
  (`parent.ReceiveTick` DeltaSeconds))

(event `self.ReceiveAnyDamage`
  (params (Damage :type "Float (single-precision)") (DamageType :type "DamageType Object Reference") (InstigatedBy :type "Controller Object Reference") (DamageCauser :type "Actor Object Reference"))
  (`parent.ReceiveAnyDamage` Damage null null null)
  (`|PlayMontage` (`self.Mesh`) "/Game/SpiderMinion/Animations/Anim_Hit_Montage.Anim_Hit_Montage"))

(event `ExplosionEvent`
  (`KismetSystemLibrary.Delay` 0.85)
  (for _array_element (`PrimitiveComponent.GetOverlappingActors` (`self.Capsule`) null)
    (cast `/Game/Blueprints/Enemies/BP_Enemy` _array_element
      (:`CastFailed`
        (`GameplayStatics.ApplyDamage` _array_element 100.0 null self)
        (`self.Death`)))))

(fn `Attack`
  (bind _charactermovement (`self.CharacterMovement`))
  (`parent.Attack`)
  (if (not (`self.Exploded`))
    (set `self.Exploded` true)
    (`self.ExplosionEvent`)
    (`MovementComponent.StopMovementImmediately` _charactermovement)
    (`CharacterMovementComponent.DisableMovement` _charactermovement)))

(fn `Death`
  (`parent.Death`))

(fn `UserConstructionScript`)