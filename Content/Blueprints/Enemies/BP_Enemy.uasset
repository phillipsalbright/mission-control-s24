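; Base enemy character that spawns and possesses itself with its own AI controller, takes damage, and can be set on fire.
; SetOnFire attaches a fire effect and refreshes a timer, while Tick applies periodic self-damage until it expires and plays movement audio.
; Death ragdolls the mesh, unpossesses, notifies GM_MissionControl, pays the reward to BP_Commander, then the body is destroyed after a long delay.
; Attack is an empty stub.
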(event `self.ReceiveBeginPlay`
  (bind _returnvalue (`|SpawnActorFromClass` (`self.ControllerType`) (`KismetMathLibrary.MakeTransform` (0.0 0.0 0.0)) "Undefined" "MultiplyWithRoot" null null))
  (`Controller.Possess` _returnvalue self))

(event `self.ReceiveAnyDamage`
  (params (Damage :type "Float (single-precision)") (DamageType :type "DamageType Object Reference") (InstigatedBy :type "Controller Object Reference") (DamageCauser :type "Actor Object Reference"))
  (bind _output_get (set `self.Health` (- (`self.Health`) Damage)))
  (if (<= _output_get 0.0)
    (if (not (`self.Dead`))
      (`self.Death`)
      (`KismetSystemLibrary.Delay` 130.0)
      (`self.K2_DestroyActor`))))

(event `self.ReceiveTick`
  (params (DeltaSeconds :type "Float (single-precision)"))
  (bind _firetimer (`self.FireTimer`))
  (bind _firedamagetimer (`self.FireDamageTimer`))
  (bind _audio (`self.Audio`))
  (`|ExecutionSequence`
    (:`then_0`
      ;[1 1 1] On Fire stuff
      (if (> _firetimer 0.0)
        (bind _output_get (set `self.FireTimer` (- _firetimer DeltaSeconds)))
        (if (> _output_get 0.0)
          (if (<= _firedamagetimer 0.0)
            (`GameplayStatics.ApplyDamage` self 5.0 null self)
            (set `self.FireDamageTimer` 0.5)
            (else
              (set `self.FireDamageTimer` (- _firedamagetimer DeltaSeconds))))
          (else
            (`self.K2_DestroyActor` (`self.FireEffect`))))))
    (:`then_1`
      (if (and (> (`KismetMathLibrary.VSizeXY` (`CharacterMovementComponent.GetLastUpdateVelocity` (`self.CharacterMovement`))) 10.0) (not (`self.Dead`)))
        (if (not (`AudioComponent.IsPlaying` _audio))
          (`AudioComponent.Play` _audio 0.0))
        (else
          (`AudioComponent.Stop` _audio))))))

(fn `Attack`)

(fn `Death`
  (bind _mesh (`self.Mesh`))
  (`CharacterMovementComponent.DisableMovement` (`self.CharacterMovement`))
  (`PrimitiveComponent.SetSimulatePhysics` _mesh true)
  (`PrimitiveComponent.SetCollisionEnabled` _mesh "QueryAndPhysics")
  (`PrimitiveComponent.SetCollisionEnabled` (`self.CapsuleComponent`) "NoCollision")
  (set `self.Dead` true)
  (`Controller.UnPossess` (`self.GetController`))
  (bind _asgm_mission_control (cast `/Game/Blueprints/GameModes/GM_MissionControl` (`GameplayStatics.GetGameMode`)))
  (`/Game/Blueprints/GameModes/GM_MissionControl.EnemyDied` _asgm_mission_control)
  (bind _returnvalue (`GameplayStatics.GetActorOfClass` "/Game/Blueprints/Players/BP_Commander.BP_Commander_C"))
  (`/Game/Blueprints/Players/BP_Commander.AddCurrency` _returnvalue (`self.Reward`)))

(fn `SetOnFire`
  (bind _mesh (`self.Mesh`))
  (if (not (> (`self.FireTimer`) 0.0))
    (bind _returnvalue (`|SpawnActorFromClass` "/Game/StarterContent/Blueprints/Blueprint_Effect_Fire.Blueprint_Effect_Fire_C" (`SceneComponent.K2_GetComponentToWorld` _mesh) "Undefined" "OverrideRootScale" null null))
    (`self.K2_AttachToComponent` _returnvalue _mesh "root" "SnapToTarget" "SnapToTarget" "KeepWorld" true)
    (set `self.FireEffect` _returnvalue))
  (set `self.FireTimer` 5.0))

(fn `SpawnBloodEffect`
  (params (Location :type "Vector Structure") (Direction :type "Vector Structure"))
  (`NiagaraFunctionLibrary.SpawnSystemAtLocation` (`self.BloodEffect`) Location (`KismetMathLibrary.Conv_VectorToRotator` Direction) (0.2 0.2 0.2)))

(fn `UserConstructionScript`)