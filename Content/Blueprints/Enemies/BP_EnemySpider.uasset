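; Spider enemy Blueprint that layers its own animations and a melee attack onto inherited enemy behavior.
; It plays montages on spawn and when damaged, while death simply defers to the parent.
; When its cooldown has expired, Attack plays a montage and immediately damages actors overlapping the capsule, skipping other BP_Enemy actors.
; The cooldown counts down on Tick and restarts only when damage is applied.
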(event `self.ReceiveBeginPlay`
  (`parent.ReceiveBeginPlay`)
  (`|PlayMontage` (`self.Mesh`) "/Game/SpiderMinion/Animations/Anim_Enter_Montage.Anim_Enter_Montage"))

(event `self.ReceiveTick`
  (params (DeltaSeconds :type "Float (single-precision)"))
  (bind _attacktimer (`self.AttackTimer`))
  (`parent.ReceiveTick` DeltaSeconds)
  (if (> _attacktimer 0.0)
    (set `self.AttackTimer` (- _attacktimer DeltaSeconds))))

(event `self.ReceiveAnyDamage`
  (params (Damage :type "Float (single-precision)") (DamageType :type "DamageType Object Reference") (InstigatedBy :type "Controller Object Reference") (DamageCauser :type "Actor Object Reference"))
  (`parent.ReceiveAnyDamage` Damage null null null)
  (`|PlayMontage` (`self.Mesh`) "/Game/SpiderMinion/Animations/Anim_Hit_Montage.Anim_Hit_Montage"))

(fn `Attack`
  (`parent.Attack`)
  (if (<= (`self.AttackTimer`) 0.0)
    (`self.PlayAnimMontage` "/Game/SpiderMinion/Animations/Anim_Attack_Montage.Anim_Attack_Montage")
    (for _array_element (`PrimitiveComponent.GetOverlappingActors` (`self.Capsule`) null)
      (cast `/Game/Blueprints/Enemies/BP_Enemy` _array_element
        (:`CastFailed`
          (`GameplayStatics.ApplyDamage` _array_element 11.0 null self)
          (set `self.AttackTimer` 1.4))))))

(fn `Death`
  (`parent.Death`))

(fn `UserConstructionScript`)