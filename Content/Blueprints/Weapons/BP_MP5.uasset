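; BP_MP5 is a weapon Blueprint for an MP5 that extends a parent weapon class by overriding its Shoot function.
; Shoot calls the parent, then plays the first-person rifle montage, a firing sound and an attached Niagara muzzle flash at the shoot point.
; It casts a bullet with set inaccuracy, damage and range, then spawns a 9mm casing at the ejection point and pushes it outward with an impulse.
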(fn `NewFunction_0`)

(fn `Shoot`
  (bind _shootpoint (`self.ShootPoint`))
  (bind _ejection (`self.ejection`))
  (`parent.Shoot`)
  (`AnimInstance.Montage_Play` (`SkeletalMeshComponent.GetAnimInstance` (`/Game/Blueprints/Players/BP_FPSCharacter.FirstPersonMesh` (`self.Character`))) "/Game/FirstPersonArms/Animations/FP_Rifle_Shoot_Montage.FP_Rifle_Shoot_Montage" 1.0 "MontageLength" 0.0 true)
  (`GameplayStatics.PlaySoundAtLocation` "/Game/FPWeapon/Audio/FirstPersonTemplateWeaponFire02.FirstPersonTemplateWeaponFire02" (`SceneComponent.K2_GetComponentLocation` _shootpoint) (struct) 1.0 1.0 0.0 null null null null) ; Play firing sound
  (`NiagaraFunctionLibrary.SpawnSystemAttached` "/Game/VFX/NS_MuzzleFlashEffect.NS_MuzzleFlashEffect" _shootpoint "None" (0.0 0.0 0.0) (struct) "KeepRelativeOffset" true)
  (`self.CastBullet` 2.5 10.0 10000.0)
  (bind _returnvalue (`|SpawnActorFromClass` "/Game/Blueprints/Weapons/BP_Ejected9mm.BP_Ejected9mm_C" (`SceneComponent.K2_GetComponentToWorld` _ejection) "Undefined" "MultiplyWithRoot" null null))
  (`PrimitiveComponent.AddImpulse` (`/Game/Blueprints/Weapons/BP_EjectedBullet.StaticMesh` _returnvalue) (* (`SceneComponent.GetForwardVector` _ejection) 40.0) "None" false))

(fn `UserConstructionScript`
  (`parent.UserConstructionScript`))