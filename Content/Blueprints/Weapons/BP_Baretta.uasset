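; Beretta pistol weapon Blueprint that overrides its parent's Shoot to add pistol-specific firing.
; After the parent call, Shoot plays the first-person arms montage, a fire sound and an attached Niagara muzzle flash at ShootPoint.
; It then calls CastBullet with fixed inaccuracy, damage and range, and plays the pistol mesh's shoot montage.
; Event graph events are disabled stubs and NewFunction_0 is empty.
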(fn `NewFunction_0`)

(fn `Shoot`
  (bind _shootpoint (`self.ShootPoint`))
  (`parent.Shoot`)
  (`AnimInstance.Montage_Play` (`SkeletalMeshComponent.GetAnimInstance` (`/Game/Blueprints/Players/BP_FPSCharacter.FirstPersonMesh` (`self.Character`))) "/Game/Models/Arms/FPSArms_Anim_Arms_Rig_Single_Arms_Shoot_Montage.FPSArms_Anim_Arms_Rig_Single_Arms_Shoot_Montage" 1.0 "MontageLength" 0.0 true)
  (`GameplayStatics.PlaySoundAtLocation` "/Game/FPWeapon/Audio/FirstPersonTemplateWeaponFire02.FirstPersonTemplateWeaponFire02" (`SceneComponent.K2_GetComponentLocation` _shootpoint) (struct) 1.0 1.0 0.0 null null null null) ; Play firing sound
  (`NiagaraFunctionLibrary.SpawnSystemAttached` "/Game/VFX/NS_MuzzleFlashEffect.NS_MuzzleFlashEffect" _shootpoint "None" (0.0 0.0 0.0) (struct) "KeepRelativeOffset" true)
  (`self.CastBullet` 1.8 20.0 10000.0)
  (`AnimInstance.Montage_Play` (`SkeletalMeshComponent.GetAnimInstance` (`self.Pistol`)) "/Game/Models/RiggedGuns/Pistol_Anim_Armature_Shoot_Montage.Pistol_Anim_Armature_Shoot_Montage" 1.0 "MontageLength" 0.0 true))

(fn `UserConstructionScript`
  (`parent.UserConstructionScript`))