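; Weapon Blueprint that holds ammo, reload and durability state, with functions to equip, unequip and shoot.
; On BeginPlay it hides and deactivates its root component and creates a WBP_WeaponHUD widget with the weapon image and zeroed ammo.
; Equip and Unequip toggle root visibility and activation.
; CanShoot requires magazine ammo and no reload in progress, while Shoot only decrements magazine ammo and durability.
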(event `self.ReceiveBeginPlay`
  (bind _defaultsceneroot (`self.DefaultSceneRoot`))
  (`ActorComponent.SetActive` _defaultsceneroot false false)
  (`SceneComponent.SetVisibility` _defaultsceneroot false true)
  (bind _returnvalue (`|CreateWidget` "/Game/UI/WBP_WeaponHUD.WBP_WeaponHUD_C"))
  (`/Game/UI/WBP_WeaponHUD.SetImage` _returnvalue (`self.WeaponImage`))
  (`/Game/UI/WBP_WeaponHUD.SetAmmo` _returnvalue 0 0))

(fn `CanShoot`
  (returns (CanShoot :type Boolean))
  (return (and (> (`self.MagAmmo`) 0) (not (`self.Reloading`)))))

(fn `Equip`
  (bind _defaultsceneroot (`self.DefaultSceneRoot`))
  (`ActorComponent.SetActive` _defaultsceneroot true false)
  (`SceneComponent.SetVisibility` _defaultsceneroot true true))

(fn `Shoot`
  (set `self.Durability` (- (`self.Durability`) (`self.DurabilityPerShot`)))
  (`/Engine/EditorBlueprintResources/StandardMacros.DecrementInt` (`self.MagAmmo`)))

(fn `Unequip`
  (bind _defaultsceneroot (`self.DefaultSceneRoot`))
  (`ActorComponent.SetActive` _defaultsceneroot false false)
  (`SceneComponent.SetVisibility` _defaultsceneroot false true))

(fn `UserConstructionScript`)