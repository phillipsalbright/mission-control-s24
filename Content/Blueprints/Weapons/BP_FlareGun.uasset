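; BP_FlareGun is a weapon Blueprint for a flare gun that fires projectiles.
; Its Shoot override calls the parent, plays montages on the first-person arms and gun body, plays a fire sound, and spawns BP_FlareProjectile at ShootPoint.
; Muzzle flash and CastBullet hitscan nodes are left unconnected and never run.
; The event graph, construction script and NewFunction_0 add no logic.
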(fn `NewFunction_0`)

(fn `Shoot`
  (`parent.Shoot`)
  (`AnimInstance.Montage_Play` (`SkeletalMeshComponent.GetAnimInstance` (`/Game/Blueprints/Players/BP_FPSCharacter.FirstPersonMesh` (`self.Character`))) "/Game/Models/Arms/FPSArms_Anim_Arms_Rig_Single_Arms_Shoot_Montage.FPSArms_Anim_Arms_Rig_Single_Arms_Shoot_Montage" 1.0 "MontageLength" 0.0 true)
  (`GameplayStatics.PlaySoundAtLocation` "/Game/FPWeapon/Audio/FirstPersonTemplateWeaponFire02.FirstPersonTemplateWeaponFire02" (`SceneComponent.K2_GetComponentLocation` (`self.ShootPoint`)) (struct) 1.0 1.0 0.0 null null null null) ; Play firing sound
  (`|SpawnActorFromClass` "/Game/Blueprints/Weapons/BP_FlareProjectile.BP_FlareProjectile_C" (`SceneComponent.K2_GetComponentToWorld` (`self.ShootPoint`)) "Undefined" "MultiplyWithRoot" null null)
  (`AnimInstance.Montage_Play` (`SkeletalMeshComponent.GetAnimInstance` (`self.FlareGun_Body`)) "/Game/Models/RiggedGuns/FlareGun_Body_Anim_Armature_Shoot_Montage.FlareGun_Body_Anim_Armature_Shoot_Montage" 1.0 "MontageLength" 0.0 true))

(fn `UserConstructionScript`
  (`parent.UserConstructionScript`))