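; BP_FlareProjectile is a flare projectile that sets BP_Enemy actors on fire.
; On BeginPlay it launches its physics-simulated StaticMesh forward by setting linear velocity.
; A Sphere overlap with an enemy ignites it and destroys the flare, ignoring other actors.
; A mesh hit on anything destroys the flare, igniting it first if it is an enemy.
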(event `self.ReceiveBeginPlay`
  (bind _staticmesh (`self.StaticMesh`))
  (`PrimitiveComponent.SetPhysicsLinearVelocity` _staticmesh (* (`SceneComponent.GetForwardVector` _staticmesh) 2000.0) false "None"))

(event `self.Sphere.OnComponentBeginOverlap`
  (params (OverlappedComponent :type "PrimitiveComponent Object Reference") (OtherActor :type "Actor Object Reference") (OtherComp :type "PrimitiveComponent Object Reference") (OtherBodyIndex :type Integer) (bFromSweep :type Boolean) (SweepResult :type "HitResult Structure (by ref)"))
  (bind _asbp_enemy (cast `/Game/Blueprints/Enemies/BP_Enemy` OtherActor))
  (`/Game/Blueprints/Enemies/BP_Enemy.SetOnFire` _asbp_enemy)
  (`self.K2_DestroyActor`))

(event `self.StaticMesh.OnComponentHit`
  (params (HitComponent :type "PrimitiveComponent Object Reference") (OtherActor :type "Actor Object Reference") (OtherComp :type "PrimitiveComponent Object Reference") (NormalImpulse :type "Vector Structure") (Hit :type "HitResult Structure (by ref)"))
  (bind _asbp_enemy (cast `/Game/Blueprints/Enemies/BP_Enemy` OtherActor)
    (:`then`
      (`/Game/Blueprints/Enemies/BP_Enemy.SetOnFire` _asbp_enemy))
    (:`CastFailed`
      _))
  (`self.K2_DestroyActor`))

(fn `UserConstructionScript`)