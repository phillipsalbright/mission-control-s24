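; BP_Revolver is a hitscan-style revolver weapon that builds on a parent weapon class.
; Its Shoot override calls the parent, plays a first-person fire montage (reusing the rifle's), a firing sound and an attached Niagara muzzle flash at the shoot point.
; It then calls the inherited CastBullet with its own inaccuracy, damage and range.
; The event graph and construction script add no behavior, and NewFunction_0 is an empty stub.
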(fn `NewFunction_0`)

(fn `Shoot`
  (bind _shootpoint (`self.ShootPoint`))
  (`parent.Shoot`)
  (`AnimInstance.Montage_Play` (`SkeletalMeshComponent.GetAnimInstance` (`/Game/Blueprints/Players/BP_FPSCharacter.FirstPersonMesh` (`self.Character`))) "/Game/FirstPersonArms/Animations/FP_Rifle_Shoot_Montage.FP_Rifle_Shoot_Montage" 1.0 "MontageLength" 0.0 true)
  (`GameplayStatics.PlaySoundAtLocation` "/Game/FPWeapon/Audio/FirstPersonTemplateWeaponFire02.FirstPersonTemplateWeaponFire02" (`SceneComponent.K2_GetComponentLocation` _shootpoint) (struct) 1.0 1.0 0.0 null null null null) ; Play firing sound
  (`NiagaraFunctionLibrary.SpawnSystemAttached` "/Game/VFX/NS_MuzzleFlashEffect.NS_MuzzleFlashEffect" _shootpoint "None" (0.0 0.0 0.0) (struct) "KeepRelativeOffset" true)
  (`self.CastBullet` 2.8 50.0 10000.0))

(fn `UserConstructionScript`
  (`parent.UserConstructionScript`))