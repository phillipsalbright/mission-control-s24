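; Ammo pickup actor that grants a configurable type and amount of ammo to the FPS player character.
; Each tick the static mesh bobs on a sine of the actor's lifetime around its starting height and spins steadily in yaw.
; When a BP_FPSCharacter overlaps the sphere, it adds the ammo through that character's inventory component and destroys itself.
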(event `self.ReceiveBeginPlay`
  (bind (_returnvalue_x _returnvalue_y _returnvalue_z) (`KismetMathLibrary.BreakVector` (`SceneComponent.K2_GetComponentLocation` (`self.StaticMesh`))))
  (set `self.BaseHeight` _returnvalue_z))

(event `self.ReceiveTick`
  (params (DeltaSeconds :type "Float (single-precision)"))
  (bind _staticmesh (`self.StaticMesh`))
  (bind (_returnvalue_roll _returnvalue_pitch _returnvalue_yaw) (`KismetMathLibrary.BreakRotator` (`SceneComponent.K2_GetComponentRotation` (`self.StaticMesh`))))
  (bind (_returnvalue_x _returnvalue_y _returnvalue_z) (`KismetMathLibrary.BreakVector` (`SceneComponent.K2_GetComponentLocation` _staticmesh)))
  (`SceneComponent.K2_SetWorldLocation` _staticmesh (`KismetMathLibrary.MakeVector` _returnvalue_x _returnvalue_y (+ (`self.BaseHeight`) (* (`KismetMathLibrary.Sin` (`self.GetGameTimeSinceCreation`)) 15.0))) false false)
  (`SceneComponent.K2_SetWorldRotation` _staticmesh (`KismetMathLibrary.MakeRotator` _returnvalue_roll _returnvalue_pitch (+ _returnvalue_yaw (* DeltaSeconds 50.0))) false false))

(event `self.Sphere.OnComponentBeginOverlap`
  (params (OverlappedComponent :type "PrimitiveComponent Object Reference") (OtherActor :type "Actor Object Reference") (OtherComp :type "PrimitiveComponent Object Reference") (OtherBodyIndex :type Integer) (bFromSweep :type Boolean) (SweepResult :type "HitResult Structure (by ref)"))
  (bind _asbp_fpscharacter (cast `/Game/Blueprints/Players/BP_FPSCharacter` OtherActor))
  (`/Game/Blueprints/Players/BP_InventoryComponent.AddAmmo` (`/Game/Blueprints/Players/BP_FPSCharacter.BP_InventoryComponent` _asbp_fpscharacter) (`self.AmmoToAdd`) (`self.AmmoAmmountToAdd`))
  (`self.K2_DestroyActor`))

(fn `UserConstructionScript`)