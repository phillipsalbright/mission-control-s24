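; Automated turret that, while active, targets living BP_Enemy actors inside its ViewCone and shoots them.
; Tick uses Delays to pace turning, firing and retargeting, with a recursive search skipping dead overlaps.
; Shots are visibility line traces from the barrel tip that apply damage and spawn effects, with debug drawing.
; ActivateTurret starts audio and an ActiveTime timer, while ModifyTurretPower temporarily swaps damage and fire delay.
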(event `self.ReceiveBeginPlay`)

(event `self.ReceiveTick`
  (params (DeltaSeconds :type "Float (single-precision)"))
  (bind _localenemy (`self.localEnemy`))
  (if (`self.Active`)
    (`/Engine/EditorBlueprintResources/StandardMacros.IsValid` _localenemy
      (:`Is Valid`
        (if (`/Game/Blueprints/Enemies/BP_Enemy.Dead` _localenemy)
          ;[1 1 1] change target if old one died, shoot every shootDelay seconds and update enemy every updateDelay seconds
          (`self.UpdateEnemyTarget` 0)
          (else
            (`KismetSystemLibrary.Delay` (`self.shootDelay`))
            (`self.Turn and Shoot Enemies`)
            (`KismetSystemLibrary.Delay` (`self.targetUpdateDelay`))
            (`self.UpdateEnemyTarget` 0)
            (`KismetSystemLibrary.PrintString` "delayUpdate"))))
      (:`Is Not Valid`
        (`self.UpdateEnemyTarget` 0)))))

(event `ModifyTurretPower`
  (params (Duration :type "Float (double-precision)") (NewDamage :type "Float (double-precision)") (NewAttackSpeed :type "Float (double-precision)") (oldDamage :type "Float (double-precision)") (oldAttackSpeed :type "Float (double-precision)"))
  (set `self.damageVal` NewDamage)
  (set `self.shootDelay` NewAttackSpeed)
  (`KismetSystemLibrary.Delay` Duration)
  (set `self.damageVal` oldDamage)
  (set `self.shootDelay` oldAttackSpeed))

(event `DeactivateTurret`
  (`AudioComponent.Stop` (`self.Audio`))
  (set `self.Active` false))

(event `self.ViewCone.OnComponentBeginOverlap`
  (params (OverlappedComponent :type "PrimitiveComponent Object Reference") (OtherActor :type "Actor Object Reference") (OtherComp :type "PrimitiveComponent Object Reference") (OtherBodyIndex :type Integer) (bFromSweep :type Boolean) (SweepResult :type "HitResult Structure (by ref)"))
  (bind _localenemy (`self.localEnemy`))
  (bind _asbp_enemy (cast `/Game/Blueprints/Enemies/BP_Enemy` OtherActor)
    (:`then`
      (if (`/Game/Blueprints/Enemies/BP_Enemy.Dead` _asbp_enemy)
        (`KismetSystemLibrary.PrintString` "targetAlreadyDead")
        (else
          (`/Engine/EditorBlueprintResources/StandardMacros.IsValid` _localenemy
            (:`Is Valid`
              ;[1 1 1] set new enemey if old one is dead or doesn't exist
              (if (`/Game/Blueprints/Enemies/BP_Enemy.Dead` _localenemy)
                (set `self.localEnemy` _asbp_enemy)
                (`KismetSystemLibrary.PrintString` "ValidTurretTargetSet")))
            (:`Is Not Valid`
              (set `self.localEnemy` _asbp_enemy)
              (`KismetSystemLibrary.PrintString` "InvalidTarget"))))))
    (:`CastFailed`
      (`KismetSystemLibrary.PrintString` (`KismetStringLibrary.Concat_StrStr` "TirretEntryCastFailed: " (`KismetSystemLibrary.GetDisplayName` OtherActor))))))

(event `self.ViewCone.OnComponentEndOverlap`
  (params (OverlappedComponent :type "PrimitiveComponent Object Reference") (OtherActor :type "Actor Object Reference") (OtherComp :type "PrimitiveComponent Object Reference") (OtherBodyIndex :type Integer))
  (bind _asbp_enemy (cast `/Game/Blueprints/Enemies/BP_Enemy` OtherActor))
  (if (== _asbp_enemy (`self.localEnemy`))
    (`self.UpdateEnemyTarget` 0)))

(fn `ActivateTurret`
  (`KismetSystemLibrary.K2_SetTimerDelegate` (`|CreateDelegate` :!event `DeactivateTurret`) (`self.activeTime`))
  (`AudioComponent.Play` (`self.Audio`) 0.0)
  (set `self.Active` true))

(fn `ShootTurret`
  (bind _barreltip (`self.BarrelTip`))
  (bind _barreltip_2 (`self.BarrelTip`))
  (bind _returnvalue (`SceneComponent.K2_GetComponentLocation` _barreltip))
  (bind _returnvalue_2 (+ _returnvalue (* (`SceneComponent.GetForwardVector` _barreltip) 10000.0)))
  (`NiagaraFunctionLibrary.SpawnSystemAtLocation` "/Game/VFX/NS_MuzzleFlashEffect.NS_MuzzleFlashEffect" (`SceneComponent.K2_GetComponentLocation` _barreltip_2) (`SceneComponent.K2_GetComponentRotation` _barreltip_2))
  (`GameplayStatics.PlaySoundAtLocation` "/Game/FPWeapon/Audio/FirstPersonTemplateWeaponFire02_Cue.FirstPersonTemplateWeaponFire02_Cue" (`SceneComponent.K2_GetComponentLocation` (`self.BarrelTip`)) (struct) 1.0 1.0 0.0 null null null null)
  (bind _outhit (`KismetSystemLibrary.LineTraceSingle` :`Start` _returnvalue :`End` _returnvalue_2 :`TraceChannel` "TraceTypeQuery1" :`bTraceComplex` true :`DrawDebugType` "ForDuration" :`DrawTime` 2.0))
  (bind _asbp_enemy (cast `/Game/Blueprints/Enemies/BP_Enemy` (`.HitActor` (`GameplayStatics.BreakHitResult` _outhit)))
    (:`then`
      (`KismetSystemLibrary.PrintString` (`KismetStringLibrary.Concat_StrStr` "turretShotAt: " (`KismetSystemLibrary.GetDisplayName` (`.HitActor` (`GameplayStatics.BreakHitResult` _outhit)))))
      (`GameplayStatics.ApplyDamage` _asbp_enemy (`self.damageVal`) null self)
      (`/Game/Blueprints/Enemies/BP_Enemy.SpawnBloodEffect` _asbp_enemy (`.Location` (`GameplayStatics.BreakHitResult` _outhit)) (`.Normal` (`GameplayStatics.BreakHitResult` _outhit)))
      (bind _asskeletal_mesh_component (cast `SkeletalMeshComponent` (`.HitComponent` (`GameplayStatics.BreakHitResult` _outhit))))
      (if (`SceneComponent.IsSimulatingPhysics` _asskeletal_mesh_component "None")
        (`PrimitiveComponent.AddImpulse` _asskeletal_mesh_component (* _returnvalue_2 (* 0.0 4000.0)) (`.HitBoneName` (`GameplayStatics.BreakHitResult` _outhit)) false)))
    (:`CastFailed`
      (`KismetSystemLibrary.PrintString` (`KismetStringLibrary.Concat_StrStr` "turretCastFailed: " (`KismetSystemLibrary.GetDisplayName` (`.HitActor` (`GameplayStatics.BreakHitResult` _outhit)))))
      (if (`GameplayStatics.BreakHitResult` _outhit)
        (`NiagaraFunctionLibrary.SpawnSystemAtLocation` "/Game/VFX/NS_DustSpray.NS_DustSpray" (`.Location` (`GameplayStatics.BreakHitResult` _outhit)) (`KismetMathLibrary.Conv_VectorToRotator` (`.Normal` (`GameplayStatics.BreakHitResult` _outhit))) (0.5 0.5 0.5))))))

(fn `Turn and Shoot Enemies`
  (bind _localenemy (`self.localEnemy`))
  ;[1 1 1] turn turret towards enemy
  (`/Engine/EditorBlueprintResources/StandardMacros.IsValid` _localenemy
    (:`Is Valid`
      (`SceneComponent.K2_SetWorldRotation` (`self.TurretChamberHOlder`) (`KismetMathLibrary.ComposeRotators` (`KismetMathLibrary.FindLookAtRotation` (`SceneComponent.K2_GetComponentLocation` (`self.BarrelTip`)) (`self.K2_GetActorLocation` _localenemy)) (`self.rotationOffset`)) false false)
      (`self.ShootTurret`))))

(fn `UpdateEnemyTarget`
  (params (index :type Integer))
  (bind _asbp_enemy (cast `/Game/Blueprints/Enemies/BP_Enemy` (`|GetArrayItem` (`PrimitiveComponent.GetOverlappingActors` (`self.ViewCone`) "/Game/Blueprints/Enemies/BP_Enemy.BP_Enemy_C") index)))
  (`/Engine/EditorBlueprintResources/StandardMacros.IsValid` _asbp_enemy
    (:`Is Valid`
      (if (`/Game/Blueprints/Enemies/BP_Enemy.Dead` _asbp_enemy)
        (`self.UpdateEnemyTarget` (+ index 1))
        (else
          (set `self.localEnemy` _asbp_enemy))))))

(fn `UserConstructionScript`)